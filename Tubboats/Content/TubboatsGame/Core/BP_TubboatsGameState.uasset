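; Game state Blueprint for Tubboats that exposes match state changes, game start, player death and remaining time.
; State changes are broadcast as gameplay messages on Event.GameState.Changed, and its own listener prints each new state for debugging.
; StartGame moves the match from Menu to PreGame, while an interface event lets other objects set the state.
; Death handling and the timer getter forward to inherited functions.
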(event `self.ReceiveBeginPlay`
  (bind (_asynctaskproxy _actualchannel _payload) (`|AsyncAction_ListenForGameplayMessages` (struct :`TagName` "Event.GameState.Changed") "/Script/Tubboats.GameStateMessage")
    (:`OnMessageReceived`
      (`KismetSystemLibrary.PrintText` (`|FormatText` "TB_GAME_STATE: {0}" (`|GetEnumeratorNameAsString` (`.GameState` (break `GameStateMessage` _payload))))))))

(event `self.BP_OnGameStateChanged`
  (params (InState :type "ETubboatGameState Enum (by ref)" :default "Menu"))
  (`GameplayMessageSubsystem.K2_BroadcastMessage` (subsystem `GameplayMessageSubsystem`) (struct :`TagName` "Event.GameState.Changed") (make `GameStateMessage` InState)))

(event `self.StartGame`
  (if (`|EnumEquality` (`self.CurrentGameState`) "Menu")
    (`self.SetGameStateFromBP` "PreGame")))

(event `self.PlayerDie`
  (params (KillingPawn :type "Pawn Object Reference"))
  (`self.PlayerDied` KillingPawn))

(event `self.SetGameStateFromBP`
  (params (NewState :type "ETubboatGameState Enum" :default "Menu"))
  (`self.SetCurrentGameState` NewState))

(fn `GetGameTimerSeconds`
  (returns (Seconds :type "Float (double-precision)"))
  (return (`self.GetCurrentRemainingTime`)))

(fn `UserConstructionScript`)