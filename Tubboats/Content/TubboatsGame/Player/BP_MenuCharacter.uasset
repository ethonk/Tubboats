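; Menu character for Tubboats that views the menu through a camera and relays boat input for two players.
; Shortly after possession it switches the view to the first actor tagged MenuCamera, and BeginPlay adds the Enhanced Input mapping context.
; The start action notifies the game state.
; Separate P1 and P2 move and fire actions broadcast through GameplayMessageSubsystem channels with a player index, so one character serves both players.
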(event `EnterMenuCamera`
  (params (InController :type "PlayerController Object Reference"))
  (bind _outactors (`GameplayStatics.GetAllActorsWithTag` "MenuCamera"))
  (if (`KismetArrayLibrary.Array_IsValidIndex` _outactors)
    (`PlayerController.SetViewTargetWithBlend` InController (`|GetArrayItem` _outactors) 0.0 "VTBlend_Linear" 0.0 false)
    (else
      (`KismetSystemLibrary.PrintString` "ba"))))

(event `self.ReceivePossessed`
  (params (NewController :type "Controller Object Reference"))
  (`KismetSystemLibrary.Delay` 0.2)
  (bind _asplayer_controller (cast `PlayerController` NewController))
  (`self.EnterMenuCamera` _asplayer_controller))

(event `self.ReceiveBeginPlay`
  (bind _asplayer_controller (cast `PlayerController` (`self.GetController`)))
  (bind _returnvalue (pcsubsystem `EnhancedInputLocalPlayerSubsystem` _asplayer_controller))
  (`/Engine/EditorBlueprintResources/StandardMacros.IsValid` _returnvalue
    (:`Is Valid`
      (`EnhancedInputSubsystemInterface.AddMappingContext` _returnvalue "/Game/TubboatsGame/Input/IMC_TubboatsInputMap.IMC_TubboatsInputMap" 0 (struct)))))

(event `EnhancedInput|/Game/TubboatsGame/Input/IA_StartGame`
  (params (ActionValue :type Boolean) (ElapsedSeconds :type "Float (double-precision)") (TriggeredSeconds :type "Float (double-precision)") (InputAction :type "InputAction Object Reference" :default "/Game/TubboatsGame/Input/IA_StartGame.IA_StartGame"))
  (bind _returnvalue (`GameplayStatics.GetGameState`))
  (:`Completed`
    (`/Engine/EditorBlueprintResources/StandardMacros.IsValid` _returnvalue
      (:`Is Valid`
        (message `/Game/TubboatsGame/Core/BPI_TubboatGameState.StartGame` _returnvalue)))))

(event `EnhancedInput|/Game/TubboatsGame/Input/IA_FireLeft`
  (params (ActionValue :type Boolean) (ElapsedSeconds :type "Float (double-precision)") (TriggeredSeconds :type "Float (double-precision)") (InputAction :type "InputAction Object Reference" :default "/Game/TubboatsGame/Input/IA_FireLeft.IA_FireLeft"))
  (:`Completed`
    (`GameplayMessageSubsystem.K2_BroadcastMessage` (subsystem `GameplayMessageSubsystem`) (struct :`TagName` "Player.Input.Fire.Left") (make `/Game/TubboatsGame/Input/S_InputMessage` 0))))

(event `EnhancedInput|/Game/TubboatsGame/Input/IA_FireLeftP2`
  (params (ActionValue :type Boolean) (ElapsedSeconds :type "Float (double-precision)") (TriggeredSeconds :type "Float (double-precision)") (InputAction :type "InputAction Object Reference" :default "/Game/TubboatsGame/Input/IA_FireLeftP2.IA_FireLeftP2"))
  (:`Completed`
    (`GameplayMessageSubsystem.K2_BroadcastMessage` (subsystem `GameplayMessageSubsystem`) (struct :`TagName` "Player.Input.Fire.Left") (make `/Game/TubboatsGame/Input/S_InputMessage` 1))))

(event `EnhancedInput|/Game/TubboatsGame/Input/IA_FireRight`
  (params (ActionValue :type Boolean) (ElapsedSeconds :type "Float (double-precision)") (TriggeredSeconds :type "Float (double-precision)") (InputAction :type "InputAction Object Reference" :default "/Game/TubboatsGame/Input/IA_FireRight.IA_FireRight"))
  (:`Completed`
    (`GameplayMessageSubsystem.K2_BroadcastMessage` (subsystem `GameplayMessageSubsystem`) (struct :`TagName` "Player.Input.Fire.Right") (make `/Game/TubboatsGame/Input/S_InputMessage` 0))))

(event `EnhancedInput|/Game/TubboatsGame/Input/IA_FireRightP2`
  (params (ActionValue :type Boolean) (ElapsedSeconds :type "Float (double-precision)") (TriggeredSeconds :type "Float (double-precision)") (InputAction :type "InputAction Object Reference" :default "/Game/TubboatsGame/Input/IA_FireRightP2.IA_FireRightP2"))
  (:`Completed`
    (`GameplayMessageSubsystem.K2_BroadcastMessage` (subsystem `GameplayMessageSubsystem`) (struct :`TagName` "Player.Input.Fire.Right") (make `/Game/TubboatsGame/Input/S_InputMessage` 1))))

(event `EnhancedInput|/Game/TubboatsGame/Input/IA_MoveP2`
  (params (ActionValue :type "Vector2D Structure") (ElapsedSeconds :type "Float (double-precision)") (TriggeredSeconds :type "Float (double-precision)") (InputAction :type "InputAction Object Reference" :default "/Game/TubboatsGame/Input/IA_MoveP2.IA_MoveP2"))
  (:`Triggered`
    (`GameplayMessageSubsystem.K2_BroadcastMessage` (subsystem `GameplayMessageSubsystem`) (struct :`TagName` "Player.Input.Move") (make `/Game/TubboatsGame/Input/S_InputMessage` 1 ActionValue))))

(event `EnhancedInput|/Game/TubboatsGame/Input/IA_Move`
  (params (ActionValue :type "Vector2D Structure") (ElapsedSeconds :type "Float (double-precision)") (TriggeredSeconds :type "Float (double-precision)") (InputAction :type "InputAction Object Reference" :default "/Game/TubboatsGame/Input/IA_Move.IA_Move"))
  (:`Triggered`
    (`KismetSystemLibrary.PrintString` (`KismetStringLibrary.Conv_Vector2dToString` ActionValue))
    (`GameplayMessageSubsystem.K2_BroadcastMessage` (subsystem `GameplayMessageSubsystem`) (struct :`TagName` "Player.Input.Move") (make `/Game/TubboatsGame/Input/S_InputMessage` 0 ActionValue))))

(fn `UserConstructionScript`)