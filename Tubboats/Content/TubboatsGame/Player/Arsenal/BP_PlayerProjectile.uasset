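; BP_PlayerProjectile is a player-fired projectile in Tubboats that knocks out other players' bubbles.
; On initialize it sets its ProjectileMovement maximum, initial and forward local velocity from ProjectileSpeed.
; A capsule overlap with another owner's active BP_PlayerBubble deactivates that bubble and destroys the projectile.
; It passes through its owner's bubble and inactive bubbles, and is destroyed on overlapping any actor that is not a bubble.
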(event `self.BP_OnInitialize`
  (bind _projectilemovement (`self.ProjectileMovement`))
  (bind _projectilespeed (`self.ProjectileSpeed`))
  (set `ProjectileMovementComponent.MaxSpeed` _projectilespeed _projectilemovement)
  (set `ProjectileMovementComponent.InitialSpeed` _projectilespeed _projectilemovement)
  (`ProjectileMovementComponent.SetVelocityInLocalSpace` (`self.ProjectileMovement`) (`KismetMathLibrary.MakeVector` (`self.ProjectileSpeed`))))

(event `self.Capsule.OnComponentBeginOverlap`
  (params (OverlappedComponent :type "PrimitiveComponent Object Reference") (OtherActor :type "Actor Object Reference") (OtherComp :type "PrimitiveComponent Object Reference") (OtherBodyIndex :type Integer) (bFromSweep :type Boolean) (SweepResult :type "HitResult Structure (by ref)"))
  (bind _asbp_player_bubble (cast `/Game/TubboatsGame/Player/Arsenal/BP_PlayerBubble` OtherActor)
    (:`then`
      (if (!= (`PlayerOwnedActor.OwnerPlayerPawn` _asbp_player_bubble) (`self.OwnerPlayerPawn`))
        (if (`PlayerBubble.bActivated` _asbp_player_bubble)
          (`PlayerBubble.SetActivated` _asbp_player_bubble false)
          (`self.K2_DestroyActor` :!label _label))))
    (:`CastFailed`
      (goto _label))))

(fn `UserConstructionScript`)