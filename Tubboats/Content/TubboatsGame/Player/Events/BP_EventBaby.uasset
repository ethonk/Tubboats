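; Event actor for the "baby" hazard in Tubboats, which reports a boat pawn it hits to the game state as a player death.
; On start it records the distance between the event mesh and a cylinder indicator, plus the indicator's scale.
; Each tick the indicator grows toward that scale as the gap closes, then hides once the remaining fraction reaches AcceptanceRadius.
; The bubble-hit handler is empty, and movement is not handled here.
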(event `self.BP_EventHitActor`
  (params (HitActor :type "Actor Object Reference"))
  (`self.OnHit_Bubble` HitActor)
  (`self.OnHit_Player` HitActor))

(event `self.BP_EventStarted`
  (set `self.StartingDistance` (`KismetMathLibrary.Vector_Distance` (`SceneComponent.K2_GetComponentLocation` (`self.EventMesh`)) (`SceneComponent.K2_GetComponentLocation` (`self.Cylinder`))))
  (set `self.StartingIndicatorScale` (`SceneComponent.K2_GetComponentScale` (`self.Cylinder`))))

(event `self.ReceiveTick`
  (params (DeltaSeconds :type "Float (single-precision)"))
  (bind _outpercent (`self.GetBabyDistancePercent`))
  (bind _cylinder (`self.Cylinder`))
  (`SceneComponent.SetWorldScale3D` (`self.Cylinder`) (* (`self.StartingIndicatorScale`) (- 1.0 _outpercent)))
  (if (<= _outpercent (`self.AcceptanceRadius`))
    (if (`SceneComponent.IsVisible` _cylinder)
      (`SceneComponent.SetVisibility` _cylinder false false))))

(fn `GetBabyDistancePercent`
  (returns (OutPercent :type "Float (double-precision)"))
  (return (/ (`KismetMathLibrary.Vector_Distance` (`SceneComponent.K2_GetComponentLocation` (`self.EventMesh`)) (`SceneComponent.K2_GetComponentLocation` (`self.Cylinder`))) (`self.StartingDistance`))))

(fn `OnHit_Bubble`
  (params (InActor :type "Actor Object Reference")))

(fn `OnHit_Player`
  (params (InActor :type "Actor Object Reference"))
  (bind _asboat_pawn (cast `BoatPawn` InActor))
  (message `/Game/TubboatsGame/Core/BPI_TubboatGameState.PlayerDie` (`GameplayStatics.GetGameState`) _asboat_pawn))

(fn `UserConstructionScript`)