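; BP_Boat is a player boat that responds to input delivered as gameplay messages.
; On BeginPlay it registers listeners for fire-left, fire-right and move channels, each carrying an S_InputMessage.
; Each handler acts only when the message's player index matches the boat's own.
; Fire messages trigger the matching side of BoatCannon, while move messages only print their 2D vector.
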(event `self.ReceiveBeginPlay`
  (bind (_asynctaskproxy _actualchannel _payload) (`|AsyncAction_ListenForGameplayMessages` (struct :`TagName` "Player.Input.Fire.Left") "/Game/TubboatsGame/Input/S_InputMessage.S_InputMessage")
    (:`then`
      (bind (_asynctaskproxy_2 _actualchannel_2 _payload_2) (`|AsyncAction_ListenForGameplayMessages` (struct :`TagName` "Player.Input.Fire.Right") "/Game/TubboatsGame/Input/S_InputMessage.S_InputMessage")
        (:`then`
          (bind (_asynctaskproxy_3 _actualchannel_3 _payload_3) (`|AsyncAction_ListenForGameplayMessages` (struct :`TagName` "Player.Input.Move") "/Game/TubboatsGame/Input/S_InputMessage.S_InputMessage")
            (:`OnMessageReceived`
              (if (`self.InputMessageMatchesPlayer` _payload_3)
                (`KismetSystemLibrary.PrintString` (`KismetStringLibrary.Conv_Vector2dToString` (`.OptionalVector2D_5_2B845E1D466315D7A98FB89E2408D7B9` (break `/Game/TubboatsGame/Input/S_InputMessage` _payload_3))))))))
        (:`OnMessageReceived`
          (if (`self.InputMessageMatchesPlayer` _payload_2)
            (`BoatCannonComponent.FireRight` (`self.BoatCannon`))))))
    (:`OnMessageReceived`
      (if (`self.InputMessageMatchesPlayer` _payload)
        (`BoatCannonComponent.FireLeft` (`self.BoatCannon`))))))

(fn `InputMessageMatchesPlayer`
  (params (S_InputMessage :type "/Game/TubboatsGame/Input/S_InputMessage Structure (by ref)"))
  (returns (Matches :type Boolean))
  (return (== (`.PlayerIndex_2_2A80BC544C5DDDA5ACE162BE042D25D8` (break `/Game/TubboatsGame/Input/S_InputMessage` S_InputMessage)) (`self.PlayerIndex`))))

(fn `UserConstructionScript`)