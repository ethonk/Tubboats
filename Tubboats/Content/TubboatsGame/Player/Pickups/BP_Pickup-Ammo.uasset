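; Ammo pickup for the Tubboats game that refills the collecting boat's cannon.
; Its OnPickup event validates the collecting actor and its CannonComponent, then sets the cannon's ammo to that component's MaxAmmo.
; An invalid actor or missing component only prints a debug message.
; BeginPlay, overlap and Tick are disabled stubs, and the construction script just calls the parent.
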(event `self.BP_OnPickup`
  (params (OtherActor :type "BoatPawn Object Reference"))
  (bind _cannoncomponent (`BoatPawn.CannonComponent` OtherActor))
  (`/Engine/EditorBlueprintResources/StandardMacros.IsValid` OtherActor
    (:`Is Valid`
      (`/Engine/EditorBlueprintResources/StandardMacros.IsValid` _cannoncomponent
        (:`Is Valid`
          (`BoatCannonComponent.SetAmmo` _cannoncomponent (`BoatCannonComponent.MaxAmmo` _cannoncomponent)))
        (:`Is Not Valid`
          (`KismetSystemLibrary.PrintString` "bad cannon componen"))))
    (:`Is Not Valid`
      (`KismetSystemLibrary.PrintString` "bad pawn"))))

(fn `UserConstructionScript`
  (`parent.UserConstructionScript`))