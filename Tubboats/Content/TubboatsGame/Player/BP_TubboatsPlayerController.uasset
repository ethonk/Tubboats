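; Player controller for Tubboats that shows the menu widget and frames the view with a menu camera.
; BeginPlay creates the configured menu widget class for the first player controller and adds it to the viewport.
; On possess, EnterMenuCamera finds actors tagged MenuCamera and sets the first one as the view target, if any exists.
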(event `self.ReceiveBeginPlay`
  (bind _returnvalue (`|CreateWidget` (`self.MenuWidgetClass`) (`GameplayStatics.GetPlayerController` 0)))
  (`UserWidget.AddToViewport` _returnvalue 0))

(event `self.ReceivePossess`
  (params (PossessedPawn :type "Pawn Object Reference"))
  (`self.EnterMenuCamera`))

(event `EnterMenuCamera`
  (bind _outactors (`GameplayStatics.GetAllActorsWithTag` "MenuCamera"))
  (if (`KismetArrayLibrary.Array_IsValidIndex` _outactors)
    (`self.SetViewTargetWithBlend` (`|GetArrayItem` _outactors))))

(fn `UserConstructionScript`)