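; Bubble health component for Tubboats player boats that reports bubble loss to the rest of the game.
; When all bubbles pop, it passes the owning BP_Boat to the game state's PlayerDieMessage.
; When the bubble count changes, it broadcasts the active count and the boat's player index on the Player.Feedback.Bubbles channel through the Gameplay Message Subsystem.
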(event `self.BP_AllBubblesPopped`
  (bind _returnvalue (`self.GetOwner`))
  (`/Engine/EditorBlueprintResources/StandardMacros.IsValid` _returnvalue
    (:`Is Valid`
      (bind _asbp_boat (cast `/Game/TubboatsGame/Player/BP_Boat` _returnvalue))
      (message `/Game/TubboatsGame/Core/BPI_TubboatGameState.PlayerDie` (`GameplayStatics.GetGameState`) _asbp_boat))))

(event `self.BP_BubbleCountChanged`
  (params (ActiveBubbleCount :type "Integer (by ref)"))
  (bind _asboat_pawn (cast `BoatPawn` (`self.GetOwner`)))
  (`GameplayMessageSubsystem.K2_BroadcastMessage` (subsystem `GameplayMessageSubsystem`) (struct :`TagName` "Player.Feedback.Bubbles") (make `/Game/TubboatsGame/Interface/S_IntValue` (`BoatPawn.PlayerIndex` _asboat_pawn) ActiveBubbleCount)))